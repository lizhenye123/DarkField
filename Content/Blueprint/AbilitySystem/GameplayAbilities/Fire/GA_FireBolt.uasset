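; GA_FireBolt is a gameplay ability that casts a fire bolt projectile toward the location under the mouse.
; On valid target data, it takes the hit location and turns the avatar toward it through CombatInterface.
; It then plays the cast montage and spawns the projectile at that target when the montage's FireBolt gameplay event arrives.
; EndAbility is not wired, so this graph never ends the ability.
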(event `self.K2_ActivateAbility`
  (bind (_asynctaskproxy _data) (`TargetDataUnderMouse.CreateTargetDataUnderMouse`)
    (:`ValidData`
      (bind _output_get (set `self.Projectile Target Location` (`.Location` (`GameplayStatics.BreakHitResult` (`AbilitySystemBlueprintLibrary.GetHitResultFromTargetData` _data)))))
      (bind _ascombat_interface (cast `CombatInterface` (`self.GetAvatarActorFromActorInfo`)))
      (`CombatInterface.UpdateFacingTarget` _ascombat_interface _output_get)
      (`AbilityTask_PlayMontageAndWait.CreatePlayMontageAndWaitProxy` "None" "/Game/Assets/Characters/Aura/Animations/Abilities/AM_Cast_FireBolt.AM_Cast_FireBolt"
        (:`then`
          (`AbilityTask_WaitGameplayEvent.WaitGameplayEvent` (struct :`TagName` "Event.Montage.FireBolt") null
            (:`EventReceived`
              (`self.SpawnProjectile` (`self.Projectile Target Location`)))))))))