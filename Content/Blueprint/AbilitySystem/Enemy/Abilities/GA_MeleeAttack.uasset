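; GA_MeleeAttack is an enemy gameplay ability that plays a random melee attack montage and damages nearby hostile players.
; It turns the avatar toward its combat target through CombatInterface, then waits for a gameplay event matching the montage's tag.
; On that event it sweeps a small radius around the tag's combat socket, damages non-friendly live players, and ends.
; The ability also ends when the montage finishes or is interrupted, or when no montages exist.
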(event `self.K2_ActivateAbility`
  (bind _returnvalue (`self.GetAvatarActorFromActorInfo`))
  (bind _returnvalue_2 (`self.GetAvatarActorFromActorInfo`))
  (bind (_taggedmontage_montage _taggedmontage_montagetag) (break `TaggedMontage` (`self.TaggedMontage`)))
  (bind _returnvalue_3 (message `EnemyInterface.GetCombatTarget` _returnvalue))
  (bind _ascombat_interface (cast `CombatInterface` _returnvalue))
  (`CombatInterface.UpdateFacingTarget` _ascombat_interface (`Actor.K2_GetActorLocation` _returnvalue_3))
  (bind _returnvalue_4 (`CombatInterface.GetAttackMontages` _ascombat_interface))
  (if (`KismetArrayLibrary.Array_IsValidIndex` _returnvalue_4)
    (set `self.TaggedMontage` (`KismetArrayLibrary.Array_Random` _returnvalue_4))
    (`AbilityTask_PlayMontageAndWait.CreatePlayMontageAndWaitProxy` "None" _taggedmontage_montage 1.0 "None" false
      (:`then`
        (`AbilityTask_WaitGameplayEvent.WaitGameplayEvent` _taggedmontage_montagetag null
          (:`EventReceived`
            (bind _returnvalue_5 (message `CombatInterface.GetCombatSocketLocation` _returnvalue_2 _taggedmontage_montagetag))
            (bind _outoverlappingactors (`AuraAbilitySystemLibrary.GetLivePlayerWithinRadius` _returnvalue_2 (`|MakeArray` _returnvalue_2) 45.0 _returnvalue_5))
            (for _array_element _outoverlappingactors
              (if (`AuraAbilitySystemLibrary.IsNotFirend` (`self.GetAvatarActorFromActorInfo`) _array_element)
                (`self.CauseDamage` _array_element)))
            (`self.K2_EndAbility`))))
      (:`OnCompleted`
        (`self.K2_EndAbility` :!label _label))
      (:`OnInterrupted`
        (goto _label))
      (:`OnCancelled`
        (goto _label)))
    (else
      (`self.K2_EndAbility`))))