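; BP_FadeActor is a static mesh actor that fades out and back in when it blocks the camera.
; Construction caches the original materials and builds dynamic instances from a separate fade material array.
; FideOut swaps in those instances and plays a timeline driving their Fade parameter, while Fidein reverses it.
; At full fade-in original materials return; if BlockVisibility is set, Visibility collision becomes Ignore when faded out and Block when restored.
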(event `/Game/Blueprint/Actor/FadeActor/I_FideInterface.FideOut`
  ;[1 1 1] 物体的阻挡相机时的淡入淡出
  (`self.SetMaterialsToDynamicInstances`)
  (bind (_direction _fide) (`Timeline|FideTimeLine` :!label _label)
    (:`Update`
      (for _array_element (`self.Dynamic Material Instance`)
        (`MaterialInstanceDynamic.SetScalarParameterValue` _array_element "Fade" _fide)))
    (:`Finished`
      (`self.FadeFinish` _fide))))

(event `/Game/Blueprint/Actor/FadeActor/I_FideInterface.FideIn`
  ;[1 1 1] 物体的阻挡相机时的淡入淡出
  (goto _label :!via `Reverse`))

(fn `FadeFinish`
  (params (`Input Pin` :type "Float (double-precision)"))
  (if (>= `Input Pin` 1.0)
    (`self.ResetMaterial`)
    (if (`self.Block Visibility`)
      (`PrimitiveComponent.SetCollisionResponseToChannel` (`self.StaticMesh`) "ECC_Visibility" "ECR_Block"))
    (elif (<= `Input Pin` 0.0)
      (if (`self.Block Visibility`)
        (`PrimitiveComponent.SetCollisionResponseToChannel` (`self.StaticMesh`) "ECC_Visibility" "ECR_Ignore")))))

(fn `ResetMaterial`
  (for (_array_element _array_index) (`self.Original Material`)
    (`PrimitiveComponent.SetMaterial` (`self.StaticMesh`) _array_index _array_element)))

(fn `SetMaterialsToDynamicInstances`
  (for (_array_element _array_index) (`self.Dynamic Material Instance`)
    (`PrimitiveComponent.SetMaterial` (`self.StaticMesh`) _array_index _array_element)))

(fn `UserConstructionScript`
  (`KismetArrayLibrary.Array_Clear` (`self.Dynamic Material Instance`))
  (set `self.Original Material` (`MeshComponent.GetMaterials` (`self.StaticMesh`)))
  (for _array_element (`self.FadeMaterialInstance`)
    (bind _returnvalue (`KismetMaterialLibrary.CreateDynamicMaterialInstance` _array_element))
    (`KismetArrayLibrary.Array_AddUnique` (`self.Dynamic Material Instance`) _returnvalue)))