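; Flame pillar actor that makes its point light flicker like fire.
; On BeginPlay it randomly picks one of two intensity timelines, so separate pillars can flicker with different patterns.
; Each timeline update sets the light intensity to the curve value scaled by BaseIntensity.
; The random choice happens only at BeginPlay, and the construction script is empty.
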(event `self.ReceiveBeginPlay`
  ;[1 1 1] 灯光的闪烁
  (`self.RandomFlameIntensity`))

(event `RandomFlameIntensity`
  ;[1 1 1] 灯光的闪烁
  (switch `int` (`KismetMathLibrary.RandomIntegerInRange` 0 1)
    (:`0`
      (`self.StartTimeline_1`))
    (:`1`
      (`self.StartTimeline_2`))))

(event `StartTimeline_1`
  ;[1 1 1] 灯光的闪烁
  (bind (_direction _newtrack_0) (`Timeline|FlameIntensityTimeline_1` :!via `PlayFromStart`)
    (:`Update`
      (`LightComponent.SetIntensity` (`self.PointLight`) (* _newtrack_0 (`self.BaseIntensity`))))))

(event `StartTimeline_2`
  ;[1 1 1] 灯光的闪烁
  (bind (_direction _newtrack_0) (`Timeline|FlameIntensityTimeline_2` :!via `PlayFromStart`)
    (:`Update`
      (`LightComponent.SetIntensity` (`self.PointLight`) (* _newtrack_0 (`self.BaseIntensity`))))))

(fn `UserConstructionScript`)